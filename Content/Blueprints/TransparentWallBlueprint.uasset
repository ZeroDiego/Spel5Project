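; Wall actor that switches its mesh between a transparent material and solid blue.
; Overlapping HideCollider makes the wall transparent, and ending the overlap restores blue, with no check on the overlapping actor.
; The H key alternates the same two materials through a looping MultiGate.
; Disconnected nodes referencing the third-person character's camera capsule and a collision check never run.
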(event OnComponentBeginOverlap(HideCollider)
  (params (OverlappedComponent :type Primitive%20Component%20Object%20Reference) (OtherActor :type Actor%20Object%20Reference) (OtherComp :type Primitive%20Component%20Object%20Reference) (OtherBodyIndex :type Integer) (bFromSweep :type Boolean) (SweepResult :type Hit%20Result%20Structure%20%28by%20ref%29))
  (Rendering|Material|SetMaterial (Variables|Default|GetStaticMeshComponent1) 0 "/Game/Gabbe/Transparent.Transparent"))

(event OnComponentEndOverlap(HideCollider)
  (params (OverlappedComponent :type Primitive%20Component%20Object%20Reference) (OtherActor :type Actor%20Object%20Reference) (OtherComp :type Primitive%20Component%20Object%20Reference) (OtherBodyIndex :type Integer))
  (Rendering|Material|SetMaterial (Variables|Default|GetStaticMeshComponent1) 0 "/Game/LevelPrototyping/Materials/MI_Solid_Blue.MI_Solid_Blue"))

(event EventBeginPlay)

(event EventTick
  (params (DeltaSeconds :type Float%20%28single-precision%29)))

(event Input|KeyboardEvents|H
  (params (Key :type Key%20Structure :default "None"))
  (bind _staticmeshcomponent1 (Variables|Default|GetStaticMeshComponent1))
  (:Pressed
    (Utilities|FlowControl|MultiGate false true -1
      (:Out%200
        (Rendering|Material|SetMaterial _staticmeshcomponent1 0 "/Game/Gabbe/Transparent.Transparent"))
      (:Out%201
        (Rendering|Material|SetMaterial _staticmeshcomponent1 0 "/Game/LevelPrototyping/Materials/MI_Solid_Blue.MI_Solid_Blue")))))

(fn ConstructionScript)