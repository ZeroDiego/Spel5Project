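; Music player actor that switches between sneak and chase music based on the ShouldChase flag of an OwnerAi actor.
; The flag is checked on BeginPlay and every Tick, triggering the matching music event.
; Each event spawns 2D sound behind a DoOnce, which resets after a random delay within the track's duration.
; Both tracks share MusicConcurrency; the chase event also calls component fade-ins, while explicit stop calls are unconnected.
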(event Custom|ChaseMusic_Event
  (bind _chasemusiccomp (Variables|Default|GetChaseMusicComp))
  (bind _sound (Variables|/Script/Engine.AudioComponent|GetSound _chasemusiccomp))
  (Utilities|FlowControl|DoOnce false :!label _label
    (:Completed
      (Audio|Components|Audio|FadeIn (Variables|Default|GetSneakMusicComp) 2.0 1.0 0.0 "Linear" :!class /Script/Engine.AudioComponent)
      (bind _returnvalue (Audio|SpawnSound2D _sound 1.0 1.0 0.0 "/Game/Gabbe/Sounds/MusicConcurrency.MusicConcurrency"))
      (Utilities|FlowControl|Delay (Math|Random|RandomFloatinRange 0.0 (Variables|/Script/Engine.SoundBase|GetDuration _sound)))
      (Audio|Components|Audio|FadeIn _chasemusiccomp 2.0 1.0 0.0 "Linear" :!class /Script/Engine.AudioComponent)
      (goto _label Reset))))

(event Custom|SneakMusic_Event
  (bind _sneakmusiccomp (Variables|Default|GetSneakMusicComp))
  (bind _sound (Variables|/Script/Engine.AudioComponent|GetSound _sneakmusiccomp))
  (Utilities|FlowControl|DoOnce false :!label _label
    (:Completed
      (bind _returnvalue (Audio|SpawnSound2D _sound 1.0 1.0 0.0 "/Game/Gabbe/Sounds/MusicConcurrency.MusicConcurrency"))
      (Utilities|FlowControl|Delay (Math|Random|RandomFloatinRange 0.0 (Variables|/Script/Engine.SoundBase|GetDuration _sound)))
      (goto _label Reset))))

(event EventBeginPlay
  (bind _returnvalue (Actor|GetActorOfClass "/Game/Erik/OwnerAi.OwnerAi_C"))
  (if (Variables|/Game/Erik/OwnerAi.OwnerAi_C|Getshould%20chase? _returnvalue)
    (CallFunction|ChaseMusicEvent)
    (else
      (CallFunction|SneakMusicEvent))))

(event Collision|EventActorBeginOverlap
  (params (OtherActor :type Actor%20Object%20Reference)))

(event EventTick
  (params (DeltaSeconds :type Float%20%28single-precision%29))
  (bind _returnvalue (Actor|GetActorOfClass "/Game/Erik/OwnerAi.OwnerAi_C"))
  (if (Variables|/Game/Erik/OwnerAi.OwnerAi_C|Getshould%20chase? _returnvalue)
    (CallFunction|ChaseMusicEvent)
    (else
      (CallFunction|SneakMusicEvent))))

(fn ConstructionScript)