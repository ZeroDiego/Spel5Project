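; Owner voice actor that picks a sound based on the state of the OwnerAi actor: hamster sighting, dog heard, or default complaining.
; BeginPlay and every Tick check ShouldChase first, then DogIsBarking, call the matching event, then print a debug label after a random Delay.
; Sounds start at random offsets; hamster and dog handlers use DoOnce with no reset, while complaints have no such gate.
; An older chained-complaint sequence remains unconnected.
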(event Custom|SeesHamster_Event
  (bind _seeshamstersound (Variables|Default|GetSeesHamsterSound))
  (bind _sound (Variables|/Script/Engine.AudioComponent|GetSound _seeshamstersound))
  (bind _duration (Variables|/Script/Engine.SoundBase|GetDuration _sound))
  (bind _returnvalue (Math|Random|RandomFloatinRange 0.0 _duration))
  (Utilities|FlowControl|DoOnce false
    (:Completed
      (Audio|Components|Audio|Play _seeshamstersound _returnvalue)
      (Utilities|FlowControl|Delay _returnvalue))))

(event Custom|HearsDog_Event
  (bind _hearsdogsound (Variables|Default|GetHearsDogSound))
  (bind _sound (Variables|/Script/Engine.AudioComponent|GetSound _hearsdogsound))
  (bind _duration (Variables|/Script/Engine.SoundBase|GetDuration _sound))
  (bind _returnvalue (Math|Random|RandomFloatinRange 0.0 _duration))
  (Utilities|FlowControl|DoOnce false
    (:Completed
      (Audio|Components|Audio|Play _hearsdogsound _returnvalue)
      (Utilities|FlowControl|Delay _returnvalue))))

(event Custom|Complain_Event
  (bind _complainsounds (Variables|Default|GetComplainSounds))
  (Audio|Components|Audio|Play _complainsounds (Math|Random|RandomFloatinRange 0.0 (Variables|/Script/Engine.SoundBase|GetDuration (Variables|/Script/Engine.AudioComponent|GetSound _complainsounds)))))

(event EventBeginPlay
  (bind _returnvalue (Actor|GetActorOfClass "/Game/Erik/OwnerAi.OwnerAi_C"))
  (if (Variables|/Game/Erik/OwnerAi.OwnerAi_C|Getshould%20chase? _returnvalue)
    (CallFunction|SeesHamsterEvent)
    (Utilities|FlowControl|Delay (Math|Random|RandomFloatinRange 0.0 (Variables|/Script/Engine.SoundBase|GetDuration (Variables|/Script/Engine.AudioComponent|GetSound (Variables|Default|GetSeesHamsterSound)))))
    (Development|PrintText "Hamster")
    (elif (Variables|/Game/Erik/OwnerAi.OwnerAi_C|GetdogIsBarking? _returnvalue)
      (CallFunction|HearsDogEvent)
      (Utilities|FlowControl|Delay (Math|Random|RandomFloatinRange 0.0 (Variables|/Script/Engine.SoundBase|GetDuration (Variables|/Script/Engine.AudioComponent|GetSound (Variables|Default|GetHearsDogSound)))))
      (Development|PrintText "Dog")
      (else
        (CallFunction|ComplainEvent)
        (Utilities|FlowControl|Delay (Math|Random|RandomFloatinRange 0.0 (Variables|/Script/Engine.SoundBase|GetDuration (Variables|/Script/Engine.AudioComponent|GetSound (Variables|Default|GetComplainSounds)))))
        (Development|PrintText "BlaBlaBla")))))

(event Collision|EventActorBeginOverlap
  (params (OtherActor :type Actor%20Object%20Reference)))

(event EventTick
  (params (DeltaSeconds :type Float%20%28single-precision%29))
  (bind _returnvalue (Actor|GetActorOfClass "/Game/Erik/OwnerAi.OwnerAi_C"))
  (if (Variables|/Game/Erik/OwnerAi.OwnerAi_C|Getshould%20chase? _returnvalue)
    (CallFunction|SeesHamsterEvent)
    (Utilities|FlowControl|Delay (Math|Random|RandomFloatinRange 0.0 (Variables|/Script/Engine.SoundBase|GetDuration (Variables|/Script/Engine.AudioComponent|GetSound (Variables|Default|GetSeesHamsterSound)))))
    (Development|PrintText "Hamster")
    (elif (Variables|/Game/Erik/OwnerAi.OwnerAi_C|GetdogIsBarking? _returnvalue)
      (CallFunction|HearsDogEvent)
      (Utilities|FlowControl|Delay (Math|Random|RandomFloatinRange 0.0 (Variables|/Script/Engine.SoundBase|GetDuration (Variables|/Script/Engine.AudioComponent|GetSound (Variables|Default|GetHearsDogSound)))))
      (Development|PrintText "Dog")
      (else
        (CallFunction|ComplainEvent)
        (Utilities|FlowControl|Delay (Math|Random|RandomFloatinRange 0.0 (Variables|/Script/Engine.SoundBase|GetDuration (Variables|/Script/Engine.AudioComponent|GetSound (Variables|Default|GetComplainSounds)))))
        (Development|PrintText "BlaBlaBla")))))

(fn ConstructionScript)