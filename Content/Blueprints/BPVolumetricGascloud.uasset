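; BPVolumetricGascloud is a gas cloud actor that appears once a gas wire is cut and a stove fan is off.
; It hides three cube components on BeginPlay.
; Two events, GasWireFillGas and StoveFanFillGas, each set their own flag and reveal the cubes only if the other flag is already set, so order does not matter.
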(event Custom|StoveFanFillGas
  (Variables|Default|SetStoveFanOff true)
  (if (Variables|Default|GetGasWireCut)
    (Rendering|SetVisibility (Variables|Default|GetCube) true false)))

(event Custom|GasWireFillGas
  (Variables|Default|SetGasWireCut true)
  (if (Variables|Default|GetStoveFanOff)
    (Rendering|SetVisibility (Variables|Default|GetCube) true false)))

(event EventBeginPlay
  (Rendering|SetVisibility (Variables|Default|GetCube) false false))

(event Collision|EventActorBeginOverlap
  (params (OtherActor :type Actor%20Object%20Reference)))

(event EventTick
  (params (DeltaSeconds :type Float%20%28single-precision%29)))

(fn ConstructionScript)