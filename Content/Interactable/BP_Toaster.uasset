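; BP_Toaster is an interactable object whose cube mesh moves with the third-person character's input while the character interacts with it.
; Box overlaps set the character's CanInteractBox flag.
; While that and IsInteractingBox are true, Tick reads the action values, with X taking priority over Y, and prints debug messages.
; SpeedDirection interpolates SMCube's relative location along its forward or right vector, scaled by signed character max speed.
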(event OnComponentBeginOverlap(Box)
  (params (OverlappedComponent :type Primitive%20Component%20Object%20Reference) (OtherActor :type Actor%20Object%20Reference) (OtherComp :type Primitive%20Component%20Object%20Reference) (OtherBodyIndex :type Integer) (bFromSweep :type Boolean) (SweepResult :type Hit%20Result%20Structure%20%28by%20ref%29))
  (Development|PrintString "CanInteract" true true "(R=0.004252,G=1.000000,B=0.000000,A=1.000000)" 2.0 "4.5")
  (Variables|/Game/ThirdPerson/Blueprints/BP_ThirdPersonCharacter.BP_ThirdPersonCharacter_C|SetCan%20Interact%20Box (Variables|Default|GetCharREF) true))

(event OnComponentEndOverlap(Box)
  (params (OverlappedComponent :type Primitive%20Component%20Object%20Reference) (OtherActor :type Actor%20Object%20Reference) (OtherComp :type Primitive%20Component%20Object%20Reference) (OtherBodyIndex :type Integer))
  (Development|PrintString "CannotInteract" true true "(R=1.000000,G=0.000000,B=0.000000,A=1.000000)" 2.0 "3.4")
  (Variables|/Game/ThirdPerson/Blueprints/BP_ThirdPersonCharacter.BP_ThirdPersonCharacter_C|SetCan%20Interact%20Box (Variables|Default|GetCharREF) false))

(event EventBeginPlay
  (bind _returnvalue (Actor|GetActorOfClass "/Game/ThirdPerson/Blueprints/BP_ThirdPersonCharacter.BP_ThirdPersonCharacter_C"))
  (Variables|Default|SetCharREF _returnvalue))

(event Collision|EventActorBeginOverlap
  (params (OtherActor :type Actor%20Object%20Reference)))

(event EventTick
  (params (DeltaSeconds :type Float%20%28single-precision%29))
  (bind _charref (Variables|Default|GetCharREF))
  (bind _charref_2 (Variables|Default|GetCharREF))
  (bind _charref_3 (Variables|Default|GetCharREF))
  (bind _charactermovement (Variables|/Script/Engine.Character|GetCharacterMovement _charref))
  (bind _action_value_y (Variables|/Game/ThirdPerson/Blueprints/BP_ThirdPersonCharacter.BP_ThirdPersonCharacter_C|GetAction%20Value%20Y _charref_2))
  (bind _action_value_x (Variables|/Game/ThirdPerson/Blueprints/BP_ThirdPersonCharacter.BP_ThirdPersonCharacter_C|GetAction%20Value%20X _charref_3))
  (bind _returnvalue (Class|MovementComponent|GetMaxSpeed _charactermovement))
  (bind _returnvalue_2 (* _returnvalue -1.0))
  (if (Variables|/Game/ThirdPerson/Blueprints/BP_ThirdPersonCharacter.BP_ThirdPersonCharacter_C|GetIs%20Interacting%20Box (Variables|Default|GetCharREF))
    (if (Variables|/Game/ThirdPerson/Blueprints/BP_ThirdPersonCharacter.BP_ThirdPersonCharacter_C|GetCan%20Interact%20Box (Variables|Default|GetCharREF))
      (Utilities|FlowControl|Sequence
        (:then_1
          (if (== _action_value_x 0.0)
            (if (== _action_value_y 0.0)
              (Development|PrintString "Is not moving forward/backwards" true true "(R=1.000000,G=0.006870,B=0.000000,A=1.000000)" 2.0 "11")
              (Variables|Default|SetIsMovingForwardBackward false)
              (elif (>= _action_value_y 0.01)
                (Development|PrintString "Is moving forward" true true "(R=0.342294,G=1.000000,B=0.000000,A=1.000000)" 2.0 "18")
                (Utilities|FlowControl|Sequence
                  (:then_0
                    (Utilities|Speed/Direction true _returnvalue))
                  (:then_1
                    (Variables|Default|SetIsMovingForwardBackward true)))
                (else
                  (Development|PrintString "Is moving backward" true true "(R=0.342294,G=1.000000,B=0.000000,A=1.000000)" 2.0 "180")
                  (Utilities|FlowControl|Sequence
                    (:then_0
                      (Utilities|Speed/Direction true _returnvalue_2))
                    (:then_1
                      (Variables|Default|SetIsMovingForwardBackward true))))))
            (elif (>= _action_value_x 0.01)
              (Development|PrintString "Is moving right" true true "(R=0.342294,G=1.000000,B=0.000000,A=1.000000)" 2.0 "18")
              (Utilities|Speed/Direction false _returnvalue)
              (else
                (Development|PrintString "Is moving left" true true "(R=0.342294,G=1.000000,B=0.000000,A=1.000000)" 2.0 "180")
                (Utilities|Speed/Direction false _returnvalue_2)))))))))

(fn ConstructionScript)