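; BP_Push2 is a pushable cube actor that only becomes physically movable while the third-person character is near it.
; Two trigger volumes, Boxx and Boxy, turn on physics simulation on the Cube when the character enters and turn it off when the character leaves.
; Each volume toggles independently, so leaving either one stops simulation even if the character remains inside the other.
; The CanPush function is an empty stub.
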(event OnComponentBeginOverlap(Boxy)
  (params (OverlappedComponent :type Primitive%20Component%20Object%20Reference) (OtherActor :type Actor%20Object%20Reference) (OtherComp :type Primitive%20Component%20Object%20Reference) (OtherBodyIndex :type Integer) (bFromSweep :type Boolean) (SweepResult :type Hit%20Result%20Structure%20%28by%20ref%29))
  (Utilities|Casting|CastToBP_ThirdPersonCharacter OtherActor)
  (Physics|SetSimulatePhysics (Variables|Default|Getcube) true))

(event OnComponentEndOverlap(Boxy)
  (params (OverlappedComponent :type Primitive%20Component%20Object%20Reference) (OtherActor :type Actor%20Object%20Reference) (OtherComp :type Primitive%20Component%20Object%20Reference) (OtherBodyIndex :type Integer))
  (Utilities|Casting|CastToBP_ThirdPersonCharacter OtherActor)
  (Physics|SetSimulatePhysics (Variables|Default|Getcube) false))

(event OnComponentBeginOverlap(Boxx)
  (params (OverlappedComponent :type Primitive%20Component%20Object%20Reference) (OtherActor :type Actor%20Object%20Reference) (OtherComp :type Primitive%20Component%20Object%20Reference) (OtherBodyIndex :type Integer) (bFromSweep :type Boolean) (SweepResult :type Hit%20Result%20Structure%20%28by%20ref%29))
  (Utilities|Casting|CastToBP_ThirdPersonCharacter OtherActor)
  (Physics|SetSimulatePhysics (Variables|Default|Getcube) true))

(event OnComponentEndOverlap(Boxx)
  (params (OverlappedComponent :type Primitive%20Component%20Object%20Reference) (OtherActor :type Actor%20Object%20Reference) (OtherComp :type Primitive%20Component%20Object%20Reference) (OtherBodyIndex :type Integer))
  (Utilities|Casting|CastToBP_ThirdPersonCharacter OtherActor)
  (Physics|SetSimulatePhysics (Variables|Default|Getcube) false))

(fn ConstructionScript)

(fn CanPush)