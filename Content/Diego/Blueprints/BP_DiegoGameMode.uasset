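; Game mode for the Diego level that shows begin and end screens and restarts the level once the dog is satisfied.
; BeginPlay adds the begin widget and caches the BP_DogCharacter found in the world.
; Tick polls the dog's satisfied state behind a one-shot boolean, then adds the end widget, waits a delay and reopens the current level by name.
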(event EventBeginPlay
  (bind _returnvalue (Game|ConstructObjectfromClass "/Game/Diego/Blueprints/WBP_DiegoBeginWidget.WBP_DiegoBeginWidget_C"))
  (UserInterface|Viewport|AddtoViewport _returnvalue 0)
  (bind _returnvalue_2 (Actor|GetActorOfClass "/Game/Diego/Blueprints/BP_DogCharacter.BP_DogCharacter_C"))
  (Class|DogComponent|SetDog (Variables|Default|GetDog) _returnvalue_2))

(event EventTick
  (params (DeltaSeconds :type Float%20%28single-precision%29))
  (if (and (Variables|Default|GetHasExecutedTickLogic) (Class|DogComponent|GetDogIsSatisfied (Variables|Default|GetDog)))
    (Variables|Default|SetHasExecutedTickLogic false)
    (bind _returnvalue (Game|ConstructObjectfromClass "/Game/Diego/Blueprints/WBP_DiegoEndWidget.WBP_DiegoEndWidget_C"))
    (UserInterface|Viewport|AddtoViewport _returnvalue 0)
    (Utilities|FlowControl|Delay (Variables|Default|GetDelayDuration))
    (bind _returnvalue_2 (Game|GetCurrentLevelName true))
    (Game|OpenLevel(byName) (Utilities|String|StringToName _returnvalue_2))))

(fn ConstructionScript)