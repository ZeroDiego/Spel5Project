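; BP_Owner is an AI owner character that walks a looping four-point patrol and can spot and chase the player.
; At each point it runs a timeline, snaps to a preset rotation, waits randomly, then moves on.
; Pawn sensing notifies the seen player once, clearing the detection message after a retriggerable delay without sightings.
; Sightings trigger an AI move toward the player only while a chase flag is set; custom events toggle it, resuming patrol when cleared.
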(event OnSeePawn(PawnSensing)
  (params (Pawn :type Pawn%20Object%20Reference))
  (Variables|Default|SetDetectedPlayer Pawn)
  (Utilities|FlowControl|Sequence
    (:then_0
      (Utilities|FlowControl|Sequence
        (:then_0
          (Utilities|FlowControl|DoOnce false :!label _label
            (:Completed
              (Class|BPIDetection|StartDetection(Message) (Variables|Default|GetDetectedPlayer) self))))
        (:then_1
          (if (Variables|Default|Getshould%20chase?)
            (CallFunction|ChasePlayer (Variables|Default|GetDetectedPlayer))))))
    (:then_1
      (Utilities|FlowControl|RetriggerableDelay 0.6)
      (Class|BPIDetection|StopDetection(Message) (Variables|Default|GetDetectedPlayer))
      (goto _label Reset))))

(event Custom|Chase%20Player
  (params (TargetActor :type Actor%20Object%20Reference))
  ;[1 1 1] Chase logik
  (AI|AIMoveTo self "3400.000000,-530.000000,90.000000" TargetActor 5.0 false
    (:OnSuccess
      (Development|PrintString "Movement worked"))
    (:OnFail
      (Development|PrintString "Movement Failed"))))

(event Custom|OwnerPatrol
  ;[1 1 1] Owner Patrol
  (Variables|/Script/Engine.CharacterMovementComponent|SetMaxWalkSpeed (Variables|Character|GetCharacterMovement) 1.5e+02)
  (AI|AIMoveTo self (Utilities|Array|Get(acopy) (Variables|Default|GetPatrolLocation) (Variables|Default|GetLocations)) 0 5.0 false
    (:OnSuccess
      (Timeline|Timeline Play
        (:Finished
          (Transformation|SetActorRotation (Math|Rotator|MakeRotator 0.0 0.0 (Utilities|Array|Get(acopy) (Variables|Default|GetRotations) (Variables|Default|GetLocations))))
          (Utilities|FlowControl|Delay (Math|Random|RandomFloatinRange 5.0 1e+01))
          (Math|Integer|IncrementInt (Variables|Default|GetLocations)
            (:%20%20
              (if (== (Variables|Default|GetLocations) 4)
                (Variables|Default|SetLocations 0)
                (CallFunction|OwnerPatrol)
                (else
                  (CallFunction|OwnerPatrol))))))))))

(event Custom|CustomEvent
  ;[1 1 1] Efter chase logik
  (Variables|Default|Setshould%20chase? false)
  (CallFunction|OwnerPatrol))

(event Custom|CustomEvent_1
  (Variables|Default|Setshould%20chase? true))

(event EventBeginPlay
  (CallFunction|OwnerPatrol))

(fn ConstructionScript)