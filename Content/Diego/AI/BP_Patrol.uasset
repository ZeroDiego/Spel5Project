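; Behavior tree task that walks the owner AI through a looping list of patrol locations, unless it is moving to death.
; On arrival it applies that stop's rotation, plays timed start, loop and end task animations, then advances the index and finishes unsuccessfully.
; Failed moves wait before advancing.
; Tick switches task animations off for chasing, moving to death or dog barking, and re-enters the animation sequence once after DeathAnimationPlayed.
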(event EventReceiveExecuteAI
  (params (OwnerController :type AI%20Controller%20Object%20Reference) (ControlledPawn :type Pawn%20Object%20Reference))
  (bind _returnvalue (Actor|GetActorOfClass "/Game/Erik/OwnerAi.OwnerAi_C"))
  (if (not (Variables|/Game/Erik/OwnerAi.OwnerAi_C|GetMovingToDeath _returnvalue))
    (Variables|Default|SetPatrolLocation (Variables|/Game/Erik/OwnerAi.OwnerAi_C|GetPatrolLocation _returnvalue))
    (AI|AIMoveTo _returnvalue (Utilities|Array|Get(acopy) (Variables|Default|GetPatrolLocation) (Variables|Default|GetLocations)) 0 5.0 false
      (:OnSuccess
        (Variables|Default|SetRotations (Variables|/Game/Erik/OwnerAi.OwnerAi_C|GetRotations _returnvalue))
        (Transformation|SetActorRotation _returnvalue (Math|Rotator|MakeRotator 0.0 0.0 (Utilities|Array|Get(acopy) (Variables|Default|GetRotations) (Variables|Default|GetLocations))))
        (Utilities|FlowControl|Delay 1.0)
        (Utilities|TaskAnimations _returnvalue))
      (:OnFail
        (Utilities|FlowControl|Delay (+ 1.83 (Variables|Default|GetChangeLocationDelay)))))
    (Math|Integer|IncrementInt (Variables|Default|GetLocations)
      (:%20%20
        (if (== (Variables|Default|GetLocations) (Utilities|Array|Length (Variables|Default|GetPatrolLocation)))
          (Variables|Default|SetLocations 0))
        (AI|BehaviorTree|FinishExecute false)))))

(event EventReceiveTickAI
  (params (OwnerController :type AI%20Controller%20Object%20Reference) (ControlledPawn :type Pawn%20Object%20Reference) (DeltaSeconds :type Float%20%28single-precision%29))
  ;[0.1302 0.1302 0.1302] Stop tasks
  (Utilities|FlowControl|Sequence
    (:then_0
      (if (Variables|/Game/Erik/OwnerAi.OwnerAi_C|GetDeathAnimationPlayed (stale EventReceiveExecuteAI _returnvalue))
        (Utilities|FlowControl|DoOnce false
          (:Completed
            (Utilities|FlowControl|Delay 1.0)
            (Utilities|TaskAnimations (stale EventReceiveExecuteAI _returnvalue))
            (Math|Integer|IncrementInt (Variables|Default|GetLocations)
              (:%20%20
                (if (== (Variables|Default|GetLocations) (Utilities|Array|Length (Variables|Default|GetPatrolLocation)))
                  (Variables|Default|SetLocations 0))
                (AI|BehaviorTree|FinishExecute false)))))))
    (:then_1
      (if (Variables|/Game/Erik/OwnerAi.OwnerAi_C|Getshould%20chase? (stale EventReceiveExecuteAI _returnvalue))
        (Default|ToggleTaskAnim (stale EventReceiveExecuteAI _returnvalue) false :!label _label)))
    (:then_2
      (if (Variables|/Game/Erik/OwnerAi.OwnerAi_C|GetMovingToDeath (stale EventReceiveExecuteAI _returnvalue))
        (goto _label)))
    (:then_3
      (if (Variables|/Game/Erik/OwnerAi.OwnerAi_C|GetdogIsBarking? (stale EventReceiveExecuteAI _returnvalue))
        (goto _label)))))