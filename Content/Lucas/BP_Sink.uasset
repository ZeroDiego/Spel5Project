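; Sink actor that triggers an owner-death ending when both the toaster and the player are in it.
; External callers set the two flags through Enable/Disable functions, and Tick polls them, firing once via DoOnce.
; The sequence blends the camera to the sink and disables character movement and camera control.
; After timed delays it kills the owner AI, shows the OwnerDeadEnd widget, then reloads the current level.
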(event EventBeginPlay
  (bind _outactors (Actor|GetAllActorsOfClass "/Game/ThirdPerson/Blueprints/BP_ThirdPersonCharacter.BP_ThirdPersonCharacter_C")))

(event EventTick
  (params (DeltaSeconds :type Float%20%28single-precision%29))
  (if (Variables|Default|GetToasterInSink)
    (if (Variables|Default|GetPlayerInSink)
      (Utilities|FlowControl|DoOnce false
        (:Completed
          (bind _outactors (Actor|GetAllActorsOfClass "BP_Sink_C"))
          (bind _array_element (Utilities|Array|ForEachLoopwithBreak _outactors :!label _label)
            (:LoopBody
              (Game|Player|SetViewTargetwithBlend (Game|GetPlayerController 0) _array_element 0.8 "VTBlend_Linear" 0.0 false)
              (goto _label Break))
            (:Completed
              (Default|CanMoveDisable (stale EventBeginPlay _outactors))
              (Default|DisableCameraMovement (stale EventBeginPlay _outactors))
              (Utilities|FlowControl|Delay 2.0)
              (Default|KillOwner (Variables|Default|GetOwnerAiREF))
              (bind _returnvalue (Game|ConstructObjectfromClass "/Game/Diego/Blueprints/OwnerDeadEnd.OwnerDeadEnd_C"))
              (UserInterface|Viewport|AddtoViewport _returnvalue 0)
              (Utilities|FlowControl|Delay 2.0)
              (bind _returnvalue_2 (Game|GetCurrentLevelName true))
              (Game|OpenLevel(byName) (Utilities|String|StringToName _returnvalue_2)))))))))

(fn ConstructionScript)

(fn EnableToasterinSink
  (Variables|Default|SetToasterInSink true))

(fn EnablePlayerinSink
  (Variables|Default|SetPlayerInSink true))

(fn DisableToasterinSink
  (Variables|Default|SetToasterInSink false))

(fn DisablePlayerinSink
  (Variables|Default|SetPlayerInSink false))