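; BP_ClimbableWall is a wall actor that highlights its mesh when the player can climb it.
; BeginPlay caches the BP_ThirdPersonCharacter, and Box overlap events set a PlayerInRange flag without checking which actor overlaps.
; Tick activates the BPHighlight on the mesh while in range and the character is not climbing, otherwise disables it.
; Both Tick branches hide InteractWidget, so the prompt never shows from this graph.
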(event OnComponentBeginOverlap(Box)
  (params (OverlappedComponent :type Primitive%20Component%20Object%20Reference) (OtherActor :type Actor%20Object%20Reference) (OtherComp :type Primitive%20Component%20Object%20Reference) (OtherBodyIndex :type Integer) (bFromSweep :type Boolean) (SweepResult :type Hit%20Result%20Structure%20%28by%20ref%29))
  (Variables|Default|SetPlayerInRange true))

(event OnComponentEndOverlap(Box)
  (params (OverlappedComponent :type Primitive%20Component%20Object%20Reference) (OtherActor :type Actor%20Object%20Reference) (OtherComp :type Primitive%20Component%20Object%20Reference) (OtherBodyIndex :type Integer))
  (Variables|Default|SetPlayerInRange false))

(event EventBeginPlay
  (bind _returnvalue (Actor|GetActorOfClass "/Game/ThirdPerson/Blueprints/BP_ThirdPersonCharacter.BP_ThirdPersonCharacter_C"))
  (Variables|Default|SetCharacterREF _returnvalue))

(event Collision|EventActorBeginOverlap
  (params (OtherActor :type Actor%20Object%20Reference)))

(event EventTick
  (params (DeltaSeconds :type Float%20%28single-precision%29))
  (bind _interactwidget (Variables|Default|GetInteractWidget))
  (bind _bp_highlight (Variables|Default|GetBP_Highlight))
  (bind _staticmesh (Variables|Default|GetStaticMesh))
  (if (Variables|Default|GetPlayerInRange)
    (if (Variables|/Game/ThirdPerson/Blueprints/BP_ThirdPersonCharacter.BP_ThirdPersonCharacter_C|GetIsClimbing? (Variables|Default|GetCharacterREF))
      (Rendering|SetVisibility _interactwidget false false :!label _label)
      (Default|DisableHighlight _bp_highlight _staticmesh)
      (else
        (Rendering|SetVisibility _interactwidget false false)
        (Default|ActivateHighlight _bp_highlight _staticmesh)))
    (else
      (goto _label))))

(fn ConstructionScript)