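; BP_Computer is an interactable computer actor that locks and releases the player's movement when used.
; Overlapping its Box highlights the mesh through BPHighlight, and leaving clears it; both paths set InteractWidget hidden.
; Interact queries the BP_ThirdPersonCharacter found at BeginPlay, then either disables movement, shows LeaveWidget and clears the highlight, or reverses all three.
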(event OnComponentBeginOverlap(Box)
  (params (OverlappedComponent :type Primitive%20Component%20Object%20Reference) (OtherActor :type Actor%20Object%20Reference) (OtherComp :type Primitive%20Component%20Object%20Reference) (OtherBodyIndex :type Integer) (bFromSweep :type Boolean) (SweepResult :type Hit%20Result%20Structure%20%28by%20ref%29))
  (Rendering|SetVisibility (Variables|Default|GetInteractWidget) false false)
  (Default|ActivateHighlight (Variables|Default|GetBP_Highlight) (Variables|Default|GetStaticMesh)))

(event OnComponentEndOverlap(Box)
  (params (OverlappedComponent :type Primitive%20Component%20Object%20Reference) (OtherActor :type Actor%20Object%20Reference) (OtherComp :type Primitive%20Component%20Object%20Reference) (OtherBodyIndex :type Integer))
  (Rendering|SetVisibility (Variables|Default|GetInteractWidget) false false)
  (Default|DisableHighlight (Variables|Default|GetBP_Highlight) (Variables|Default|GetStaticMesh)))

(event EventBeginPlay
  (bind _outactors (Actor|GetAllActorsOfClass "/Game/ThirdPerson/Blueprints/BP_ThirdPersonCharacter.BP_ThirdPersonCharacter_C"))
  (Rendering|SetVisibility (Variables|Default|GetLeaveWidget) false false))

(event Collision|EventActorBeginOverlap
  (params (OtherActor :type Actor%20Object%20Reference)))

(event EventTick
  (params (DeltaSeconds :type Float%20%28single-precision%29)))

(event EventInteract
  (params (Player :type Character%20Object%20Reference))
  (bind _leavewidget (Variables|Default|GetLeaveWidget))
  (bind _interactwidget (Variables|Default|GetInteractWidget))
  (bind _bp_highlight (Variables|Default|GetBP_Highlight))
  (bind _staticmesh (Variables|Default|GetStaticMesh))
  (bind _canmove_ (Default|CheckifCanMove (stale EventBeginPlay _outactors)))
  (if _canmove_
    (Default|CanMoveDisable (stale EventBeginPlay _outactors))
    (Rendering|SetVisibility _leavewidget true false)
    (Rendering|SetVisibility _interactwidget false false)
    (Default|DisableHighlight _bp_highlight _staticmesh)
    (else
      (Default|CanMoveEnabled (stale EventBeginPlay _outactors))
      (Rendering|SetVisibility _leavewidget false false)
      (Rendering|SetVisibility _interactwidget false false)
      (Default|ActivateHighlight _bp_highlight _staticmesh))))

(fn ConstructionScript)