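; BP_UISkinDisplay is a display actor that shows the currently selected hamster skin, likely for a UI preview.
; Every Tick it casts to BP_MainGameInstance, caches the reference and calls SkinEquip.
; SkinEquip switches on the instance's ESkinCharacter value and sets the mesh's first material to the matching hamster skin.
; The skin is polled and reapplied each frame, with no change event.
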(event Custom|Skin%20Equip
  (bind _mesh (Variables|Character|GetMesh))
  (switch Utilities|FlowControl|Switch|SwitchonE_SkinCharacter (Variables|/Game/UI/Menus/BP_MainGameInstance.BP_MainGameInstance_C|GetE_SkinCharacter (Variables|Default|GetAs%20BP%20Main%20Game%20Instance))
    (:NewEnumerator2
      (Rendering|Material|SetMaterial _mesh 0 "/Game/3DStuff/Hamster/Materials/M_HamsterSkinGinger.M_HamsterSkinGinger"))
    (:NewEnumerator0
      (Rendering|Material|SetMaterial _mesh 0 "/Game/3DStuff/Hamster/Materials/M_HamsterSkinBeige.M_HamsterSkinBeige"))
    (:NewEnumerator1
      (Rendering|Material|SetMaterial _mesh 0 "/Game/3DStuff/Hamster/Materials/M_HamsterSkinGrey.M_HamsterSkinGrey"))))

(event EventBeginPlay)

(event Collision|EventActorBeginOverlap
  (params (OtherActor :type Actor%20Object%20Reference)))

(event EventTick
  (params (DeltaSeconds :type Float%20%28single-precision%29))
  (bind _asbp_main_game_instance (Utilities|Casting|CastToBP_MainGameInstance (Game|GetGameInstance)))
  (Variables|Default|SetAs%20BP%20Main%20Game%20Instance _asbp_main_game_instance)
  (CallFunction|SkinEquip))

(fn ConstructionScript)